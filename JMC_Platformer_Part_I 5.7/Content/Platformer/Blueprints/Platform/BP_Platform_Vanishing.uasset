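; BP_Platform_Vanishing is a platform that disappears after the player stands on it for a set lifetime, then reappears.
; A trigger zone flags when player pawn 0 is on it, and Tick accumulates continuous standing time, resetting it otherwise.
; At the lifetime, it hides and disables collision, waits, then restores its BeginPlay transform, visibility and collision.
; Debug prints report overlaps and the running timer.
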(event `self.ReceiveBeginPlay`
  ; Set Start Position, Rotation & Scale
  (set `self.StartTransform` (`self.GetTransform`)))

(event `ReturnToStart`
  ;[1 1 1 0.5] Return to Start
  (`SceneComponent.K2_SetWorldTransform` (`self.DefaultSceneRoot`) (`self.StartTransform`) false true)
  (set `self.TimeOnPlatform` 0.0)
  (`self.SetActorHiddenInGame` false)
  (`self.SetActorEnableCollision` true))

(event `self.ReceiveTick`
  (params (DeltaSeconds :type "Float (single-precision)"))
  ;[0.08866 0.000911 0.15 0.502] Set Timer For Platform
  (if (`self.IsPlayerOnPlatform`)
    (bind _output_get (set `self.TimeOnPlatform` (+ (`self.TimeOnPlatform`) DeltaSeconds)))
    (`|ExecutionSequence`
      (:`then_0`
        ;[0.08866 0.000911 0.15 0.502] Check if Timer has Reached The Platform's Life Time
        (if (>= (`self.TimeOnPlatform`) (`self.PlatformLifetime`))
          ;[0.08866 0.000911 0.15 0.502] Hide & Disable Platform
          (`self.SetActorHiddenInGame` true)
          (`self.SetActorEnableCollision` false)
          (`KismetSystemLibrary.Delay` (`self.TimeInvisible`))
          (`self.ReturnToStart`)))
      (:`then_1`
        (`KismetSystemLibrary.PrintString` (`KismetStringLibrary.Conv_DoubleToString` _output_get))))
    (else
      (set `self.TimeOnPlatform` 0.0))))

(event `self.PlatformTriggerZone.OnComponentBeginOverlap`
  (params (OverlappedComponent :type "PrimitiveComponent Object Reference") (OtherActor :type "Actor Object Reference") (OtherComp :type "PrimitiveComponent Object Reference") (OtherBodyIndex :type Integer) (bFromSweep :type Boolean) (SweepResult :type "HitResult Structure (by ref)"))
  ;[0.004083 1 0 0.5] Collider Check
  (if (== OtherActor (`GameplayStatics.GetPlayerPawn` 0))
    (`|ExecutionSequence`
      (:`then_0`
        (`KismetSystemLibrary.PrintString` "PLAYER IS ON THE PLATFORM"))
      (:`then_1`
        (set `self.IsPlayerOnPlatform` true)))))

(event `self.PlatformTriggerZone.OnComponentEndOverlap`
  (params (OverlappedComponent :type "PrimitiveComponent Object Reference") (OtherActor :type "Actor Object Reference") (OtherComp :type "PrimitiveComponent Object Reference") (OtherBodyIndex :type Integer))
  ;[0.004083 1 0 0.5] Collider Check
  (if (== OtherActor (`GameplayStatics.GetPlayerPawn` 0))
    (`|ExecutionSequence`
      (:`then_0`
        (`KismetSystemLibrary.PrintString` "PLAYER IS ON THE PLATFORM"))
      (:`then_1`
        (set `self.IsPlayerOnPlatform` false)))))

(fn `UserConstructionScript`)