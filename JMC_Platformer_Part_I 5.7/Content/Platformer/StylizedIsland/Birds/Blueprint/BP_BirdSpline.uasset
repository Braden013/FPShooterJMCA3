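; Ambient bird flock actor that moves a configurable number of static mesh birds along a spline path.
; The construction script spawns the birds with random spacing, offsets and flap-rate dynamic materials.
; At BeginPlay, the BirdMovement timeline drives BirdUpdate, wrapping each bird's spline distance to set its transform.
; A BirdOffset timeline is meant to drift offsets toward random targets, but its lerp alpha is fixed at zero.
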(event `self.ReceiveBeginPlay`
  (`|ExecutionSequence`
    (:`then_0`
      (bind (_direction _lerp) (`Timeline|BirdMovement`)
        (:`Update`
          (for (_ _array_index) (`self.BirdMesh`)
            (`self.BirdUpdate` (* (`self.NumberOfLoops`) _lerp) _array_index)))))
    (:`then_1`
      (for (_ _array_index_2) (`self.BirdMesh`)
        (`KismetArrayLibrary.Array_Set` (`self.OffsetStart`) _array_index_2 (`|GetArrayItem` (`self.Offset`) _array_index_2) true)
        (`KismetArrayLibrary.Array_Set` (`self.OffsetEnd`) 0 (* (`KismetMathLibrary.RandomUnitVector`) (`self.RandomizeOffset`)) true))
      (`Timeline|BirdOffset`
        (:`Update`
          (for (_ _array_index_3) (`self.BirdMesh`)
            (`KismetArrayLibrary.Array_Set` (`self.Offset`) _array_index_3 (`KismetMathLibrary.VLerp` (`|GetArrayItem` (`self.OffsetStart`) _array_index_3) (`|GetArrayItem` (`self.OffsetEnd`) _array_index_3)))))))))

(fn `BirdUpdate`
  (params (Position :type "Float (double-precision)") (BirdIndex :type Integer))
  (bind _spline (`self.Spline`))
  (bind _returnvalue (* (`SplineComponent.GetSplineLength` _spline) (`KismetMathLibrary.Fraction` (+ Position (`|GetArrayItem` (`self.RandomSpawnLocation`) BirdIndex)))))
  (`SceneComponent.K2_SetRelativeTransform` (`|GetArrayItem` (`self.BirdMesh`) BirdIndex) (`KismetMathLibrary.MakeTransform` (+ (`SplineComponent.GetLocationAtDistanceAlongSpline` _spline _returnvalue "Local") (`|GetArrayItem` (`self.Offset`) BirdIndex)) (`SplineComponent.GetRotationAtDistanceAlongSpline` _spline _returnvalue "Local") (`KismetMathLibrary.Conv_DoubleToVector` (`self.BirdScale`))) false false))

(fn `UserConstructionScript`
  (bind _spline (`self.Spline`))
  (`SplineComponent.SetClosedLoop` (`self.Spline`) (`self.Loops`) true)
  (for _ (range (`self.BirdSpawnAmount`))
    (bind _returnvalue (`AddComponent|NODE_AddStaticMeshComponent-3`))
    (`StaticMeshComponent.SetStaticMesh` _returnvalue (`self.StaticBirdMesh`))
    (bind _returnvalue_2 (`PrimitiveComponent.CreateDynamicMaterialInstance` _returnvalue 0 "/Game/Platformer/StylizedIsland/Birds/Materials/M_BirdFlapBP.M_BirdFlapBP" "None"))
    (`KismetArrayLibrary.Array_Add` (`self.BirdMaterial`) _returnvalue_2)
    (`MaterialInstanceDynamic.SetScalarParameterValue` _returnvalue_2 "FlapCount" (`KismetMathLibrary.RandomFloatInRange` 0.9 1.25))
    (`KismetArrayLibrary.Array_Add` (`self.Offset`) (* (`KismetMathLibrary.RandomUnitVector`) (`self.RandomizeOffset`)))
    (`KismetArrayLibrary.Array_Add` (`self.RandomSpawnLocation`) (`KismetMathLibrary.RandomFloatInRange` 0.0 (`self.RandomizeStart`))))
  (bind _output_get (set `self.BirdMesh` (`self.K2_GetComponentsByClass` "/Script/Engine.StaticMeshComponent")))
  (for (_ _array_index) _output_get
    (`self.BirdUpdate` (`self.StartingPosition`) _array_index)
    (if (`self.SplinePoints`)
      (for _index (range (`SplineComponent.GetNumberOfSplinePoints` _spline))
        (bind _returnvalue_3 (`AddComponent|NODE_AddStaticMeshComponent-2` :`RelativeTransform` (`SplineComponent.GetTransformAtSplinePoint` _spline _index "Local" false)))
        (`SceneComponent.SetHiddenInGame` _returnvalue_3 true false)))))